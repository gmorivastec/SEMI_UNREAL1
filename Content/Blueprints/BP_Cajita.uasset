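; BP_Cajita is a debug-style test actor with a static mesh that the player pushes using the Space Bar.
; Both press and release add a force along player controller 0's forward vector, scaled by Intensidad, and print a message that names F instead of Space.
; Construction, BeginPlay and overlaps print debug text, showing the Nombre variable and the colliding actor's name.
; Tick does nothing, as its DeltaSeconds print is disconnected.
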(event `self.ReceiveBeginPlay`
  (`KismetSystemLibrary.PrintString` (`self.nombre`)))

(event `self.ReceiveActorBeginOverlap`
  (params (OtherActor :type "Actor Object Reference"))
  (`KismetSystemLibrary.PrintString` (`KismetStringLibrary.Concat_StrStr` "Colisionando con: " (`KismetSystemLibrary.GetDisplayName` OtherActor))))

(event `self.ReceiveTick`
  (params (DeltaSeconds :type "Float (single-precision)")))

(event `Key|SpaceBar`
  (params (Key :type "Key Structure"))
  (:`Pressed`
    (`KismetSystemLibrary.PrintString` "*** PRESIONASTE F ***" :!label _label)
    (`PrimitiveComponent.AddForce` (`self.StaticMeshComponent`) (* (`self.GetActorForwardVector` (`GameplayStatics.GetPlayerController` 0)) (`self.intensidad`)) "None" false))
  (:`Released`
    (goto _label)))

(fn `UserConstructionScript`
  (`KismetSystemLibrary.PrintString` "CONSTRUCCION"))